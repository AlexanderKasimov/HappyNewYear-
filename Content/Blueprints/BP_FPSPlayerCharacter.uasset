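; First-person player character Blueprint that handles aim zoom, sprinting, door interaction and the player's HUD widget.
; Zoom toggles the aim state and hand animation, while holding Left Shift swaps walk for run speed; both adjust crosshair visibility on UI_WaveModPlayer.
; InteractZone overlaps track tagged BP_BaseDoor actors for Use to open.
; The construction script attaches a new skeletal mesh component to the first-person mesh's WeaponSocket.
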(event OnComponentBeginOverlap(InteractZone)
  (params (OverlappedComponent :type Primitive%20Component%20Object%20Reference) (OtherActor :type Actor%20Object%20Reference) (OtherComp :type Primitive%20Component%20Object%20Reference) (OtherBodyIndex :type Integer) (bFromSweep :type Boolean) (SweepResult :type Hit%20Result%20Structure%20%28by%20ref%29))
  (if (Actor|ActorHasTag OtherActor "Door")
    (bind _asbp_base_door (Utilities|Casting|CastToBP_BaseDoor OtherActor))
    (Variables|Default|SetOverlapingDoor _asbp_base_door)))

(event OnComponentEndOverlap(InteractZone)
  (params (OverlappedComponent :type Primitive%20Component%20Object%20Reference) (OtherActor :type Actor%20Object%20Reference) (OtherComp :type Primitive%20Component%20Object%20Reference) (OtherBodyIndex :type Integer))
  (if (== OtherActor (Variables|Default|GetOverlapingDoor))
    (Variables|Default|SetOverlapingDoor 0)))

(event EventBeginPlay
  (bind _returnvalue (UserInterface|CreateWidget "/Game/UI/UI_WaveModPlayer.UI_WaveModPlayer_C"))
  (bind _output_get (Variables|Default|SetUI_ref _returnvalue))
  (UserInterface|Viewport|AddtoViewport _output_get 0))

(event Collision|EventActorBeginOverlap
  (params (OtherActor :type Actor%20Object%20Reference)))

(event EventTick
  (params (DeltaSeconds :type Float%20%28single-precision%29)))

(event Input|ActionEvents|InputActionZoom
  (params (Key :type Key%20Structure))
  (:Pressed
    (Utilities|FlowControl|FlipFlop
      (:A
        (Class|FPSBasePlayerCharacter|SetWantstoZoom true)
        (Components|Animation|PlayAnimation (Variables|Default|GetMesh1P) "/Game/Meshes/SkeletalMeshes/COD/Characters/Hands_Aim.Hands_Aim" true)
        (Widget|SetVisibility (Variables|/Game/UI/UI_WaveModPlayer.UI_WaveModPlayer_C|Getdynamic_crosshair_up (Variables|Default|GetUI_ref)) "Hidden")
        (Widget|SetVisibility (Variables|/Game/UI/UI_WaveModPlayer.UI_WaveModPlayer_C|Getdynamic_crosshair_down (Variables|Default|GetUI_ref)) "Hidden")
        (Widget|SetVisibility (Variables|/Game/UI/UI_WaveModPlayer.UI_WaveModPlayer_C|Getdynamic_crosshair_left (Variables|Default|GetUI_ref)) "Hidden")
        (Widget|SetVisibility (Variables|/Game/UI/UI_WaveModPlayer.UI_WaveModPlayer_C|Getdynamic_crosshair_right (Variables|Default|GetUI_ref)) "Hidden"))
      (:B
        (Class|FPSBasePlayerCharacter|SetWantstoZoom false)
        (Components|Animation|PlayAnimation (Variables|Default|GetMesh1P) "/Game/Meshes/SkeletalMeshes/COD/Characters/Hand_08_Anim.Hand_08_Anim" true)
        (Widget|SetVisibility (Variables|/Game/UI/UI_WaveModPlayer.UI_WaveModPlayer_C|Getdynamic_crosshair_up (Variables|Default|GetUI_ref)) "Visible")
        (Widget|SetVisibility (Variables|/Game/UI/UI_WaveModPlayer.UI_WaveModPlayer_C|Getdynamic_crosshair_down (Variables|Default|GetUI_ref)) "Visible")
        (Widget|SetVisibility (Variables|/Game/UI/UI_WaveModPlayer.UI_WaveModPlayer_C|Getdynamic_crosshair_left (Variables|Default|GetUI_ref)) "Visible")
        (Widget|SetVisibility (Variables|/Game/UI/UI_WaveModPlayer.UI_WaveModPlayer_C|Getdynamic_crosshair_right (Variables|Default|GetUI_ref)) "Visible")))))

(event Input|ActionEvents|InputActionUse
  (params (Key :type Key%20Structure))
  (:Pressed
    (Utilities|IsValid (Variables|Default|GetOverlapingDoor)
      (:Is%20Valid
        (if (!= (Variables|Default|GetOverlapingDoor) 0)
          (Default|Open (Variables|Default|GetOverlapingDoor)))))))

(event Input|KeyboardEvents|LeftShift
  (params (Key :type Key%20Structure))
  (:Pressed
    (Widget|SetVisibility (Variables|/Game/UI/UI_WaveModPlayer.UI_WaveModPlayer_C|GetRunCrosshair (Variables|Default|GetUI_ref)) "Visible")
    (Widget|SetVisibility (Variables|/Game/UI/UI_WaveModPlayer.UI_WaveModPlayer_C|Getdynamic_crosshair_up (Variables|Default|GetUI_ref)) "Hidden")
    (Widget|SetVisibility (Variables|/Game/UI/UI_WaveModPlayer.UI_WaveModPlayer_C|Getdynamic_crosshair_down (Variables|Default|GetUI_ref)) "Hidden")
    (Widget|SetVisibility (Variables|/Game/UI/UI_WaveModPlayer.UI_WaveModPlayer_C|Getdynamic_crosshair_left (Variables|Default|GetUI_ref)) "Hidden")
    (Widget|SetVisibility (Variables|/Game/UI/UI_WaveModPlayer.UI_WaveModPlayer_C|Getdynamic_crosshair_right (Variables|Default|GetUI_ref)) "Hidden")
    (Variables|/Script/Engine.CharacterMovementComponent|SetMaxWalkSpeed (Variables|Character|GetCharacterMovement) (Variables|Default|GetSpeedRun)))
  (:Released
    (Widget|SetVisibility (Variables|/Game/UI/UI_WaveModPlayer.UI_WaveModPlayer_C|GetRunCrosshair (Variables|Default|GetUI_ref)) "Hidden")
    (Widget|SetVisibility (Variables|/Game/UI/UI_WaveModPlayer.UI_WaveModPlayer_C|Getdynamic_crosshair_up (Variables|Default|GetUI_ref)) "Visible")
    (Widget|SetVisibility (Variables|/Game/UI/UI_WaveModPlayer.UI_WaveModPlayer_C|Getdynamic_crosshair_down (Variables|Default|GetUI_ref)) "Visible")
    (Widget|SetVisibility (Variables|/Game/UI/UI_WaveModPlayer.UI_WaveModPlayer_C|Getdynamic_crosshair_left (Variables|Default|GetUI_ref)) "Visible")
    (Widget|SetVisibility (Variables|/Game/UI/UI_WaveModPlayer.UI_WaveModPlayer_C|Getdynamic_crosshair_right (Variables|Default|GetUI_ref)) "Visible")
    (Variables|/Script/Engine.CharacterMovementComponent|SetMaxWalkSpeed (Variables|Character|GetCharacterMovement) (Variables|Default|GetSpeedWalk))))

(fn ConstructionScript
  (bind _returnvalue (AddComponent|AddSkeletalMeshComponent false (Math|Transform|MakeTransform "0, 0, 0")))
  (Transformation|AttachComponentToComponent _returnvalue (Variables|Default|GetMesh1P) "WeaponSocket" "SnapToTarget" "SnapToTarget" "KeepRelative" true))