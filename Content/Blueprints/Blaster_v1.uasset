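; Battery-powered automatic blaster that spawns laser projectiles with sound while the trigger is held, with a laser sight and spinning barrel.
; Trigger events start and clear looping timers for firing and timeline-driven barrel rotation.
; Each shot drains the battery and colors an indicator green, yellow or red by charge; an empty battery refills instantly.
; Tick line-traces to place the sight beam's end, brightening its dynamic material on hits.
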(event Custom|Fire
  (bind _lazerspawn (Variables|Default|GetLazerSpawn))
  (bind _curbatterylevel (Variables|Default|GetCurBatteryLevel))
  (bind _returnvalue (Transformation|GetWorldTransform _lazerspawn))
  (if (< (- _curbatterylevel 1) 0)
    (CallFunction|Reload)
    (else
      (Math|Integer|CompareInt _curbatterylevel 25
        (:>
          (Rendering|Material|SetVectorParameterValue (Variables|Default|GetIndicatorMat) "BaseColor" "(R=0.000000,G=1.000000,B=0.000000,A=1.000000)" :!class /Script/Engine.MaterialInstanceDynamic))
        (:==
          (Rendering|Material|SetVectorParameterValue (Variables|Default|GetIndicatorMat) "BaseColor" "(R=1.000000,G=1.000000,B=0.000000,A=1.000000)" :!class /Script/Engine.MaterialInstanceDynamic :!label _label))
        (:<
          (Math|Integer|CompareInt _curbatterylevel 10
            (:>
              (goto _label))
            (:==
              _)
            (:<
              _))
          (Rendering|Material|SetVectorParameterValue (Variables|Default|GetIndicatorMat) "BaseColor" "(R=1.000000,G=0.000000,B=0.000000,A=1.000000)" :!class /Script/Engine.MaterialInstanceDynamic)))
      (Game|SpawnActorfromClass "/Game/Blueprints/Lazer_v1.Lazer_v1_C" _returnvalue "AlwaysSpawn" 0 0)
      (Math|Integer|DecrementInt _curbatterylevel
        (:%20%20
          (Audio|PlaySoundatLocation "/Game/Sound/InGameSound/laser_Cue.laser_Cue" (.Location (Math|Transform|BreakTransform _returnvalue))))))))

(event Custom|ReleaseTrigger
  (Utilities|Time|ClearandInvalidateTimerbyHandle (Variables|Default|GetFireTimer))
  (Utilities|Time|ClearandInvalidateTimerbyHandle (Variables|Default|GetRotationTimer))
  (Transformation|SetRelativeRotation (Variables|Default|GetStaticMesh2) "0, 0, 0" false false)
  (Utilities|FlowControl|DoOnce false) ; enters at Reset
)

(event Custom|RotateBarrel
  (bind _staticmesh2 (Variables|Default|GetStaticMesh2))
  (bind _output_get (Variables|Default|SetOldBarrelRotation (Variables|/Script/Engine.SceneComponent|GetRelativeRotation _staticmesh2)))
  (Variables|Default|SetNewBarrelRotation (Math|Rotator|MakeRotator (.Roll (Math|Rotator|BreakRotator _output_get)) (- (.Pitch (Math|Rotator|BreakRotator _output_get)) 3.6e+02) (.Yaw (Math|Rotator|BreakRotator _output_get))))
  (bind _newtrack_0 (Timeline|Timeline_0 PlayFromStart)
    (:Update
      (Transformation|SetRelativeRotation _staticmesh2 (Math|Rotator|Lerp(Rotator) (Variables|Default|GetOldBarrelRotation) (Variables|Default|GetNewBarrelRotation) _newtrack_0) false false))))

(event Custom|PullTrigger
  (Utilities|FlowControl|DoOnce false
    (:Completed
      (CallFunction|Fire)
      (CallFunction|RotateBarrel)
      (bind _returnvalue (Utilities|Time|SetTimerbyEvent (delegate Custom|Fire) 0.1 true))
      (Variables|Default|SetFireTimer _returnvalue)
      (bind _returnvalue_2 (Utilities|Time|SetTimerbyEvent (delegate Custom|RotateBarrel) 0.5 true))
      (Variables|Default|SetRotationTimer _returnvalue_2))))

(event Custom|Reload
  (Variables|Default|SetCurBatteryLevel (Variables|Default|GetBatterySize)))

(event EventBeginPlay
  (Variables|Default|SetCurBatteryLevel (Variables|Default|GetBatterySize))
  (bind _returnvalue (Rendering|Material|CreateDynamicMaterialInstance "/Game/Materials/Mat_LazerPointer_v2.Mat_LazerPointer_v2" :!class /Script/Engine.KismetMaterialLibrary))
  (bind _output_get (Variables|Default|SetLaserPointerMat _returnvalue))
  (Rendering|Material|SetScalarParameterValue _output_get "Power" 1e+01 :!class /Script/Engine.MaterialInstanceDynamic)
  (Rendering|Material|SetScalarParameterValue (Variables|Default|GetLaserPointerMat) "Opacity" 0.01 :!class /Script/Engine.MaterialInstanceDynamic)
  (Rendering|Material|SetMaterial (Variables|Default|GetParticleSystem) 0 (Variables|Default|GetLaserPointerMat)))

(event EventTick
  (params (DeltaSeconds :type Float%20%28single-precision%29))
  (bind _lazerspawn (Variables|Default|GetLazerSpawn))
  (bind _particlesystem (Variables|Default|GetParticleSystem))
  (bind _returnvalue (Transformation|GetWorldLocation _lazerspawn))
  (bind (_outhit _returnvalue_2) (Collision|LineTraceForObjects _returnvalue (+ _returnvalue (* (Math|Vector|GetForwardVector (Transformation|GetWorldRotation (Variables|Default|GetLazerSpawn))) 2e+03)) (Utilities|Array|MakeArray "ObjectTypeQuery4" "ObjectTypeQuery1") true 0 "None"))
  (if _returnvalue_2
    (Rendering|Material|SetScalarParameterValue (Variables|Default|GetLaserPointerMat) "Power" 5e+01 :!class /Script/Engine.MaterialInstanceDynamic)
    (Rendering|Material|SetScalarParameterValue (Variables|Default|GetLaserPointerMat) "Opacity" 0.5 :!class /Script/Engine.MaterialInstanceDynamic)
    (Class|ParticleSystemComponent|SetBeamTargetPoint _particlesystem 0 (.Location (Collision|BreakHitResult _outhit)))
    (else
      (Rendering|Material|SetScalarParameterValue (Variables|Default|GetLaserPointerMat) "Power" 1e+01 :!class /Script/Engine.MaterialInstanceDynamic)
      (Rendering|Material|SetScalarParameterValue (Variables|Default|GetLaserPointerMat) "Opacity" 0.01 :!class /Script/Engine.MaterialInstanceDynamic)
      (Class|ParticleSystemComponent|SetBeamTargetPoint _particlesystem 0 (Transformation|GetWorldLocation (Variables|Default|GetlazerEndPoint))))))

(fn ConstructionScript
  (bind _returnvalue (Rendering|Material|CreateDynamicMaterialInstance (Variables|Default|GetIndicator) 0 "/Game/Materials/Mat_EmissiveSwordEdge.Mat_EmissiveSwordEdge" :!class /Script/Engine.PrimitiveComponent))
  (Variables|Default|SetIndicatorMat _returnvalue)
  (Rendering|Material|SetVectorParameterValue (Variables|Default|GetIndicatorMat) "BaseColor" "(R=0.000000,G=1.000000,B=0.000000,A=1.000000)" :!class /Script/Engine.MaterialInstanceDynamic))