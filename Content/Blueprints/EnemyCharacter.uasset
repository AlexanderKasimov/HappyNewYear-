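; Melee enemy for a wave-based FPS, with randomly colored materials, a spawned helmet and a physically animated upper body.
; Hits add impulses and drain HP, while knee, elbow or neck hits break that joint and kill.
; AttackZone loops timeline-driven hand swings toward the player, with a hand sphere and line trace landing damage.
; Death ragdolls the body, drops the helmet, adds score and has the game mode check if all are dead.
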(event OnComponentBeginOverlap(AttackZone)
  (params (OverlappedComponent :type Primitive%20Component%20Object%20Reference) (OtherActor :type Actor%20Object%20Reference) (OtherComp :type Primitive%20Component%20Object%20Reference) (OtherBodyIndex :type Integer) (bFromSweep :type Boolean) (SweepResult :type Hit%20Result%20Structure%20%28by%20ref%29))
  ;[1 1 1] Refactor this shit/ It's Attacking System
  (if (Actor|ActorHasTag OtherActor "Player")
    (CallFunction|Attack)
    (bind _returnvalue (Utilities|Time|SetTimerbyEvent (delegate Custom|Attack) 1.1 true))
    (Variables|Default|SetAttackTimer _returnvalue)))

(event OnComponentBeginOverlap(rightDamageSphere)
  (params (OverlappedComponent :type Primitive%20Component%20Object%20Reference) (OtherActor :type Actor%20Object%20Reference) (OtherComp :type Primitive%20Component%20Object%20Reference) (OtherBodyIndex :type Integer) (bFromSweep :type Boolean) (SweepResult :type Hit%20Result%20Structure%20%28by%20ref%29))
  (bind _rightdamagesphere (Variables|Default|GetrightDamageSphere))
  (bind _returnvalue (Transformation|GetWorldRotation _rightdamagesphere))
  (bind _returnvalue_2 (Transformation|GetWorldLocation _rightdamagesphere))
  (bind _returnvalue_3 (Math|Vector|GetForwardVector _returnvalue))
  ;[1 1 1] Refactor this shit/ It's Attacking System
  (if (and (Actor|ActorHasTag OtherActor "Player") (Variables|Default|GetisAttacking))
    (bind (_outhit _returnvalue_4) (Collision|LineTraceForObjects (+ _returnvalue_2 (* _returnvalue_3 -2e+01)) (+ _returnvalue_2 (* _returnvalue_3 3e+01)) (Utilities|Array|MakeArray "ObjectTypeQuery4") true 0 "None"))
    (if (Actor|ActorHasTag (.HitActor (Collision|BreakHitResult _outhit)) "Player")
      (Utilities|FlowControl|DoOnce false
        (:Completed
          (if _returnvalue_4
            (Class|IDamagable|RecieveDamage(Message) (.HitActor (Collision|BreakHitResult _outhit)) _outhit (Variables|Default|GetDamage) 0.0)
            (Audio|PlaySoundatLocation "/Game/Sound/InGameSound/lasgun-impact_Cue.lasgun-impact_Cue" (.Location (Collision|BreakHitResult _outhit)))))))))

(event OnComponentEndOverlap(AttackZone)
  (params (OverlappedComponent :type Primitive%20Component%20Object%20Reference) (OtherActor :type Actor%20Object%20Reference) (OtherComp :type Primitive%20Component%20Object%20Reference) (OtherBodyIndex :type Integer))
  ;[1 1 1] Refactor this shit/ It's Attacking System
  (if (Actor|ActorHasTag OtherActor "Player")
    (Utilities|Time|ClearandInvalidateTimerbyHandle (Variables|Default|GetAttackTimer))
    (Variables|Default|SetisAttacking false)
    (Variables|Default|SetRightHandTransform (Transformation|GetWorldTransform (Variables|/Game/Blueprints/MainPlayerCharacter.MainPlayerCharacter_C|GetTarget (.AsMain%20Player%20Character (Utilities|Casting|CastToMainPlayerCharacter (Game|GetPlayerCharacter 0))))))))

(event Custom|HideScore
  (Rendering|SetVisibility (Variables|Default|GetScoreText) false false))

(event Custom|RightLeg
  ;[1 0 0.8636] Not Working
  (Class|SkeletalMeshComponent|AddImpulsetoAllBodiesBelow (Variables|Character|GetMesh) (* (Transformation|GetActorForwardVector) 3e+04) (Utilities|Name|MakeLiteralName "thigh_r") false true))

(event Custom|Attack
  ;[1 1 1] Refactor this shit/ It's Attacking System
  (Variables|Default|SetisAttacking true)
  (bind _newtrack_0 (Timeline|Timeline_0 ReverseFromEnd)
    (:Update
      (Variables|Default|SetRightHandTransform (Math|Transform|Lerp(Transform) (Transformation|GetWorldTransform (Variables|Default|GetRightHand)) (Transformation|GetWorldTransform (Variables|/Game/Blueprints/MainPlayerCharacter.MainPlayerCharacter_C|GetTarget (.AsMain%20Player%20Character (Utilities|Casting|CastToMainPlayerCharacter (Game|GetPlayerCharacter 0))))) _newtrack_0)))
    (:Finished
      (bind _newtrack_0_2 (Timeline|Timeline_1 PlayFromStart)
        (:Update
          (Variables|Default|SetRightHandTransform (Math|Transform|Lerp(Transform) (Transformation|GetWorldTransform (Variables|Default|GetRightHand)) (Transformation|GetWorldTransform (Variables|/Game/Blueprints/MainPlayerCharacter.MainPlayerCharacter_C|GetTarget (.AsMain%20Player%20Character (Utilities|Casting|CastToMainPlayerCharacter (Game|GetPlayerCharacter 0))))) _newtrack_0_2)))
        (:Finished
          (Utilities|FlowControl|DoOnce false) ; enters at Reset
        )))))

(event EventTick
  (params (DeltaSeconds :type Float%20%28single-precision%29))
  ;[1 0.9345 0] Was Rotating ScoreText
)

(event EventRecieveDamage
  (params (HitInfo :type Hit%20Result%20Structure) (Damage :type Float%20%28single-precision%29) (Speed :type Float%20%28single-precision%29))
  (bind (_bblockinghit _binitialoverlap _time _distance _location _impactpoint _normal _impactnormal _physmat _hitactor _hitcomponent _hitbonename) (Collision|BreakHitResult HitInfo))
  (bind _mesh (Variables|Character|GetMesh))
  ;[1 1 1] Refactor Too\ Recieve Damage System
  (Variables|Default|SetRecievedDamage Damage)
  (Variables|Default|SetImpactSpeed Speed)
  (Variables|Default|SetImpactLocation _location)
  (Variables|Default|SetImpactNormal _normal)
  (Variables|Default|SetHittedBoneName _hitbonename)
  (if (Math|Boolean|ORBoolean (Utilities|String|Contains (Utilities|String|ToString(Name) (Variables|Default|GetHittedBoneName)) "knee") (Utilities|String|Contains (Utilities|String|ToString(Name) (Variables|Default|GetHittedBoneName)) "elbow") (Utilities|String|Contains (Utilities|String|ToString(Name) (Variables|Default|GetHittedBoneName)) "neck"))
    (Utilities|FlowControl|Sequence
      (:then_0
        (Utilities|FlowControl|DoOnce (Variables|Default|GetIsDead?)
          (:Completed
            (CallFunction|SetDead (Variables|Default|GetImpactNormal) (Variables|Default|GetImpactSpeed)))))
      (:then_1
        (Class|SkeletalMeshComponent|BreakConstraint _mesh (* (Variables|Default|GetImpactNormal) (* (Variables|Default|GetImpactSpeed) 5.0 -1.0)) (Variables|Default|GetImpactLocation) (Variables|Default|GetHittedBoneName))
        (Physics|AddImpulse _mesh (* (Variables|Default|GetImpactNormal) (* (Variables|Default|GetImpactSpeed) 1.0 -1.0)) (Variables|Default|GetHittedBoneName) false)
        (Effects|SpawnEmitteratLocation "/Game/Effects/ParticleSystems/Gameplay/Player/P_body_bullet_impact.P_body_bullet_impact" (Variables|Default|GetImpactLocation) (Math|Conversions|RotationFromXVector (Variables|Default|GetImpactNormal)) "4.000000,4.000000,4.000000")
        (Audio|PlaySoundatLocation "/Game/Sound/InGameSound/bullet_flesh_mega_Cue.bullet_flesh_mega_Cue" (Variables|Default|GetImpactLocation))))
    (else
      (Physics|AddImpulseatLocation (Variables|Character|GetMesh) (* (Variables|Default|GetImpactNormal) (* (Variables|Default|GetImpactSpeed) 1e+01 -1.0)) (Variables|Default|GetImpactLocation) (Variables|Default|GetHittedBoneName))
      (Effects|SpawnEmitteratLocation "/Game/Effects/ParticleSystems/Gameplay/Player/P_body_bullet_impact.P_body_bullet_impact" (Variables|Default|GetImpactLocation) (Math|Conversions|RotationFromXVector (Variables|Default|GetImpactNormal)) "2.000000,2.000000,2.000000")
      (Audio|PlaySoundatLocation "/Game/Sound/InGameSound/bullet_flesh_mega_Cue.bullet_flesh_mega_Cue" (Variables|Default|GetImpactLocation) "0, 0, 0" 0.5)
      (bind _output_get (Variables|Default|SetCurHP (- (Variables|Default|GetCurHP) (Variables|Default|GetRecievedDamage))))
      (if (and (<= _output_get 0.0) (not (Variables|Default|GetIsDead?)))
        (CallFunction|SetDead (Variables|Default|GetImpactNormal) (Variables|Default|GetImpactSpeed))))))

(event EventBeginPlay
  (bind _physicalanimation (Variables|Default|GetPhysicalAnimation))
  ;[1 1 1] Some crazy physics shit
  (Utilities|FlowControl|Sequence
    (:then_0
      (Rendering|SetVisibility (Variables|Default|GetScoreText) false false)
      (Class|PhysicalAnimationComponent|SetSkeletalMeshComponent _physicalanimation (Variables|Character|GetMesh))
      (Class|PhysicalAnimationComponent|ApplyPhysicalAnimationSettingsBelow _physicalanimation (Utilities|Name|MakeLiteralName "spine_01") (Utilities|Struct|MakePhysicalAnimationData false 1e+03 1e+02 1e+03 1e+02) false)
      (Class|SkeletalMeshComponent|SetAllBodiesBelowSimulatePhysics (Variables|Character|GetMesh) (Utilities|Name|MakeLiteralName "spine_01") true false)
      (Variables|Default|SetCurHP (Variables|Default|GetMaxHP)))
    (:then_1
      (bind _returnvalue (Game|SpawnActorfromClass "/Game/Blueprints/Helmet.Helmet_C" (Transformation|GetActorTransform) "Undefined" 0 0))
      (bind _output_get (Variables|Default|SetHelmetRef _returnvalue))
      (Transformation|AttachComponentToComponent (Variables|/Game/Blueprints/Helmet.Helmet_C|GetSkeletalMesh _output_get) (Variables|Character|GetMesh) "headSocket" "SnapToTarget" "SnapToTarget" "KeepRelative" false))))

(fn ConstructionScript
  (Utilities|FlowControl|Sequence
    (:then_0
      (bind _returnvalue (AddComponent|AddSphereComponent false (Transformation|GetSocketTransform (Variables|Character|GetMesh) "rS" "RTS_Actor")))
      (bind _output_get (Variables|Default|SetrightDamageSphere _returnvalue))
      (Transformation|AttachComponentToComponent _output_get (Variables|Character|GetMesh) "rS" "SnapToTarget" "SnapToTarget" "KeepRelative" true))
    (:then_1
      (bind _returnvalue_2 (Rendering|Material|CreateDynamicMaterialInstance "/Game/Materials/Mat_BaseMat.Mat_BaseMat" :!class /Script/Engine.KismetMaterialLibrary))
      (bind _output_get_2 (Variables|Default|SetUpperBodyMat _returnvalue_2))
      (Rendering|Material|SetMaterial (Variables|Character|GetMesh) 2 _output_get_2)
      (Rendering|Material|SetMaterial (Variables|Character|GetMesh) 3 (Variables|Default|GetUpperBodyMat))
      (Rendering|Material|SetMaterial (Variables|Character|GetMesh) 7 (Variables|Default|GetUpperBodyMat))
      (Rendering|Material|SetVectorParameterValue (Variables|Default|GetUpperBodyMat) "BaseColor" (Utilities|Struct|MakeLinearColor (Math|Random|RandomFloatinRange 0.0 1.0) (Math|Random|RandomFloatinRange 0.0 1.0) (Math|Random|RandomFloatinRange 0.0 1.0) 0.0) :!class /Script/Engine.MaterialInstanceDynamic))
    (:then_2
      (bind _returnvalue_3 (Rendering|Material|CreateDynamicMaterialInstance "/Game/Materials/Mat_BaseMat.Mat_BaseMat" :!class /Script/Engine.KismetMaterialLibrary))
      (bind _output_get_3 (Variables|Default|SetHeadMat _returnvalue_3))
      (Rendering|Material|SetMaterial (Variables|Character|GetMesh) 0 _output_get_3)
      (Rendering|Material|SetVectorParameterValue (Variables|Default|GetHeadMat) "BaseColor" (Utilities|Struct|MakeLinearColor (Math|Random|RandomFloatinRange 0.0 1.0) (Math|Random|RandomFloatinRange 0.0 1.0) (Math|Random|RandomFloatinRange 0.0 1.0) 0.0) :!class /Script/Engine.MaterialInstanceDynamic))))

(fn SetDead
  (params (Normal :type Vector) (Speed :type Float%20%28single-precision%29))
  (bind _returnvalue (Game|GetGameMode))
  (bind _helmetref (Variables|Default|GetHelmetRef))
  (bind _asfps_waves_game_mode (Utilities|Casting|CastToFPS_WavesGameMode _returnvalue))
  (bind _skeletalmesh (Variables|/Game/Blueprints/Helmet.Helmet_C|GetSkeletalMesh _helmetref))
  (Variables|Default|SetisAttacking false)
  (Variables|Default|SetIsDead? true)
  (Class|PhysicalAnimationComponent|SetStrengthMultiplyer (Variables|Default|GetPhysicalAnimation) 0.0)
  (Physics|SetSimulatePhysics (Variables|Character|GetMesh) true)
  (Collision|SetCollisionEnabled (Variables|Collision|GetCapsuleComponent) "NoCollision")
  (Transformation|DetachFromActor _helmetref "KeepWorld" "KeepWorld" "KeepWorld")
  (Physics|SetSimulatePhysics _skeletalmesh true)
  (Class|SkeletalMeshComponent|SetAllBodiesBelowSimulatePhysics _skeletalmesh (Utilities|Name|MakeLiteralName "Bone") true true)
  (Collision|SetCollisionResponsetoChannel _skeletalmesh "ECC_PhysicsBody" "ECR_Block")
  (Physics|AddImpulse _skeletalmesh (* Normal (* Speed 1.0 -1.0)) "None" false)
  (Variables|/Game/Blueprints/FPS_WavesGameMode.FPS_WavesGameMode_C|SetPlayerScore _asfps_waves_game_mode (+ (Variables|/Game/Blueprints/FPS_WavesGameMode.FPS_WavesGameMode_C|GetPlayerScore _asfps_waves_game_mode) (Variables|Default|GetScore)))
  (Default|CheckIsAllDead (.AsFPS%20Waves%20Game%20Mode (Utilities|Casting|CastToFPS_WavesGameMode (Game|GetGameMode)))))