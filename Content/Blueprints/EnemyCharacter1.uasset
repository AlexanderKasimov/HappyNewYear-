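; EnemyCharacter1 is an enemy character Blueprint whose construction script is empty, so it does nothing when run.
; Disconnected, never-executed nodes would create left and right damage spheres at the mesh's "lS" and "rS" sockets.
; In that unused chain, the right sphere snaps to its socket and gets an attached arrow component, while the left sphere is only created and stored.
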(fn ConstructionScript)