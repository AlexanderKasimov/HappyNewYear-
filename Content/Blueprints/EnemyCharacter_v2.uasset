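; Zombie enemy character for a wave-based FPS, driven by a behavior tree, with a timed speed-boost charge and a hand-sphere melee attack.
; Physical animation simulates bodies below groin and thighs, so hits push bones and occasionally break constraints.
; Point damage reduces HP, flags the player's hit and spawns player-facing damage widgets.
; Death ragdolls the mesh, updates either wave game mode's score and alive check, and grants player XP.
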(event OnComponentBeginOverlap(RightHandAttackSphere)
  (params (OverlappedComponent :type Primitive%20Component%20Object%20Reference) (OtherActor :type Actor%20Object%20Reference) (OtherComp :type Primitive%20Component%20Object%20Reference) (OtherBodyIndex :type Integer) (bFromSweep :type Boolean) (SweepResult :type Hit%20Result%20Structure%20%28by%20ref%29))
  (if (Actor|ActorHasTag OtherActor "Player")
    (if (!= OtherActor (Variables|Default|GetDamagedActor))
      (Game|Damage|ApplyDamage OtherActor 25.0 0 0)
      (Variables|Default|SetDamagedActor OtherActor))))

(event Custom|HideScore
  (Rendering|SetVisibility (Variables|Default|GetScoreText) false false))

(event Custom|RightLeg
  ;[1 0 0.8636] Not Working
  (Class|SkeletalMeshComponent|AddImpulsetoAllBodiesBelow (Variables|Character|GetMesh) (* (Transformation|GetActorForwardVector) 3e+04) (Utilities|Name|MakeLiteralName "thigh_r") false true))

(event Custom|AttackStart
  (Collision|SetCollisionEnabled (Variables|Default|GetRightHandAttackSphere) "QueryOnly")
  (Variables|Default|SetDamagedActor 0))

(event Custom|AttackEnd
  (Collision|SetCollisionEnabled (Variables|Default|GetRightHandAttackSphere) "NoCollision")
  (Variables|Default|SetDamagedActor 0))

(event Custom|Charge
  (bind _charactermovement (Variables|Character|GetCharacterMovement))
  (Variables|/Script/Engine.CharacterMovementComponent|SetMaxWalkSpeed _charactermovement (+ (Variables|/Script/Engine.CharacterMovementComponent|GetMaxWalkSpeed _charactermovement) 2e+03))
  (Variables|Default|SetIsCharged? true)
  (Utilities|Time|SetTimerbyEvent (delegate Custom|StopCharge) 0.5))

(event Custom|StopCharge
  (bind _charactermovement (Variables|Character|GetCharacterMovement))
  (Variables|/Script/Engine.CharacterMovementComponent|SetMaxWalkSpeed _charactermovement (- (Variables|/Script/Engine.CharacterMovementComponent|GetMaxWalkSpeed _charactermovement) 2e+03))
  (Utilities|Time|SetTimerbyEvent (delegate Custom|ReCharge) 5.0))

(event Custom|ReCharge
  (Variables|Default|SetIsCharged? false))

(event Game|Damage|EventPointDamage
  (params (Damage :type Float%20%28single-precision%29) (DamageType :type Damage%20Type%20Object%20Reference) (HitLocation :type Vector :default "0, 0, 0") (HitNormal :type Vector :default "0, 0, 0") (HitComponent :type Primitive%20Component%20Object%20Reference) (BoneName :type Name :default "None") (ShotFromDirection :type Vector :default "0, 0, 0") (InstigatedBy :type Controller%20Object%20Reference) (DamageCauser :type Actor%20Object%20Reference) (HitInfo :type Hit%20Result%20Structure%20%28by%20ref%29))
  (bind (_bblockinghit _binitialoverlap _time _distance _location _impactpoint _normal _impactnormal _physmat _hitactor _hitcomponent _hitbonename) (Collision|BreakHitResult HitInfo))
  (bind _mesh (Variables|Character|GetMesh))
  ;[1 1 1] Refactor Too\ Recieve Damage System
  (Utilities|FlowControl|Sequence
    (:then_0
      (Variables|Default|SetRecievedDamage Damage)
      (Variables|Default|SetImpactSpeed 1e+03)
      (Variables|Default|SetImpactLocation _location)
      (Variables|Default|SetImpactNormal _normal)
      (Variables|Default|SetHittedBoneName _hitbonename)
      (if (> (Math|Random|RandomFloatinRange 0.0 1e+02) 95.0)
        (Class|PhysicalAnimationComponent|ApplyPhysicalAnimationSettingsBelow (Variables|Default|GetPhysicalAnimation) (Variables|Default|GetHittedBoneName) (Utilities|Struct|MakePhysicalAnimationData false 0.0) true)
        (Class|SkeletalMeshComponent|BreakConstraint _mesh (* (Variables|Default|GetImpactNormal) (* (Variables|Default|GetImpactSpeed) 5.0 -1.0)) (Variables|Default|GetImpactLocation) (Variables|Default|GetHittedBoneName))
        (Physics|AddImpulse _mesh (* (Variables|Default|GetImpactNormal) (* (Variables|Default|GetImpactSpeed) 1.0 -1.0)) (Variables|Default|GetHittedBoneName) false)
        (else
          (Physics|AddImpulseatLocation (Variables|Character|GetMesh) (* (Variables|Default|GetImpactNormal) (* (Variables|Default|GetImpactSpeed) 1e+01 -1.0)) (Variables|Default|GetImpactLocation) (Variables|Default|GetHittedBoneName))))
      (bind _output_get (Variables|Default|SetCurHP (- (Variables|Default|GetCurHP) (Variables|Default|GetRecievedDamage))))
      (if (and (<= _output_get 0.0) (not (Variables|Default|GetIsDead?)))
        (CallFunction|SetDead (Variables|Default|GetImpactNormal) (Variables|Default|GetImpactSpeed))))
    (:then_1
      (bind _asbp_fpsplayer_character (Utilities|Casting|CastToBP_FPSPlayerCharacter (Game|GetPlayerCharacter 0)))
      (Variables|/Game/Blueprints/BP_FPSPlayerCharacter.BP_FPSPlayerCharacter_C|SetisHitSomebody _asbp_fpsplayer_character true)
      (Utilities|FlowControl|Delay 0.2)
      (Variables|/Game/Blueprints/BP_FPSPlayerCharacter.BP_FPSPlayerCharacter_C|SetisHitSomebody _asbp_fpsplayer_character false))
    (:then_2
      (bind _returnvalue (AddComponent|AddWidgetComponent false))
      (bind _output_get_2 (Variables|Default|SetDamageTag _returnvalue))
      (Transformation|SetWorldLocation _output_get_2 (+ _location (* (Math|Rotator|GetRotationXVector (Math|Rotator|FindLookatRotation _location (Transformation|GetActorLocation (Game|GetPlayerCharacter 0)))) 5e+01)) false false)
      (bind _returnvalue_2 (UserInterface|CreateWidget "/Game/UI/UI_Damage_widget.UI_Damage_widget_C" 0 self))
      (UserInterface|SetWidget (Variables|Default|GetDamageTag) _returnvalue_2)
      (Utilities|FlowControl|Delay 3.0)
      (Components|DestroyComponent (Variables|Default|GetDamageTag)))))

(event EventTick
  (params (DeltaSeconds :type Float%20%28single-precision%29))
  (bind _damagetag (Variables|Default|GetDamageTag))
  (bind _enemytag (Variables|Default|GetEnemyTag))
  (bind _relativerotation (Variables|/Script/Engine.SceneComponent|GetRelativeRotation _damagetag))
  (bind _relativerotation_2 (Variables|/Script/Engine.SceneComponent|GetRelativeRotation _enemytag))
  (bind (_roll _pitch) (Math|Rotator|BreakRotator _relativerotation))
  (bind (_roll_2 _pitch_2) (Math|Rotator|BreakRotator _relativerotation_2))
  ;[1 0.9345 0] Was Rotating ScoreText
  (Transformation|SetWorldRotation _enemytag (Math|Rotator|MakeRotator _roll_2 _pitch_2 (.Yaw (Math|Rotator|BreakRotator (Math|Rotator|FindLookatRotation (Transformation|GetWorldLocation (Variables|Default|GetEnemyTag)) (Transformation|GetActorLocation (Game|GetPlayerCharacter 0)))))) false false)
  (Utilities|IsValid _damagetag
    (:Is%20Valid
      (Transformation|SetWorldRotation _damagetag (Math|Rotator|MakeRotator _roll _pitch (.Yaw (Math|Rotator|BreakRotator (Math|Rotator|FindLookatRotation (Transformation|GetWorldLocation (Variables|Default|GetDamageTag)) (Transformation|GetActorLocation (Game|GetPlayerCharacter 0)))))) false false))))

(event EventRecieveDamage
  (params (HitInfo :type Hit%20Result%20Structure) (Damage :type Float%20%28single-precision%29) (Speed :type Float%20%28single-precision%29)))

(event EventBeginPlay
  (bind _physicalanimation (Variables|Default|GetPhysicalAnimation))
  ;[1 1 1] Some crazy physics shit
  (Utilities|FlowControl|Sequence
    (:then_0
      (Variables|Default|SetCurHP (Variables|Default|GetMaxHP))
      (Rendering|SetVisibility (Variables|Default|GetScoreText) false false)
      (Class|PhysicalAnimationComponent|SetSkeletalMeshComponent _physicalanimation (Variables|Character|GetMesh))
      (Class|PhysicalAnimationComponent|ApplyPhysicalAnimationSettingsBelow _physicalanimation (Utilities|Name|MakeLiteralName "Groin") (Utilities|Struct|MakePhysicalAnimationData false 1e+03 1e+02 1e+03 1e+02) false)
      (Class|SkeletalMeshComponent|SetAllBodiesBelowSimulatePhysics (Variables|Character|GetMesh) (Utilities|Name|MakeLiteralName "Groin") true false)
      (Class|PhysicalAnimationComponent|ApplyPhysicalAnimationSettingsBelow (Variables|Default|GetPhysicalAnimation) (Utilities|Name|MakeLiteralName "Thigh_L") (Utilities|Struct|MakePhysicalAnimationData false 1e+03 1e+02 1e+03 1e+02) true)
      (Class|SkeletalMeshComponent|SetAllBodiesBelowSimulatePhysics (Variables|Character|GetMesh) (Utilities|Name|MakeLiteralName "Thigh_L") true true)
      (Class|PhysicalAnimationComponent|ApplyPhysicalAnimationSettingsBelow (Variables|Default|GetPhysicalAnimation) (Utilities|Name|MakeLiteralName "Thigh_R") (Utilities|Struct|MakePhysicalAnimationData false 1e+03 1e+02 1e+03 1e+02) true)
      (Class|SkeletalMeshComponent|SetAllBodiesBelowSimulatePhysics (Variables|Character|GetMesh) (Utilities|Name|MakeLiteralName "Thigh_R") true true))
    (:then_1
      (bind _returnvalue (UserInterface|CreateWidget "/Game/UI/UI_EnemyTag.UI_EnemyTag_C" 0 self))
      (UserInterface|SetWidget (Variables|Default|GetEnemyTag) _returnvalue))
    (:then_2
      (AI|RunBehaviorTree (AI|GetAIController self) "/Game/Ai/Zombie_v1/BT_Zombie_v1.BT_Zombie_v1"))
    (:then_3
      (Collision|SetCollisionEnabled (Variables|Default|GetRightHandAttackSphere) "NoCollision"))))

(fn ConstructionScript
  (Utilities|FlowControl|Sequence
    (:then_0
      (bind _returnvalue (AddComponent|AddWidgetComponent false))
      (bind _output_get (Variables|Default|SetEnemyTag _returnvalue))
      (Transformation|AttachComponentToComponent _output_get (Variables|Collision|GetCapsuleComponent) "None" "SnapToTarget" "KeepRelative" "KeepRelative" false)
      (Transformation|SetRelativeLocation (Variables|Default|GetEnemyTag) "0, 0,100.000000" false false))
    (:then_1
      (bind _returnvalue_2 (AddComponent|AddSphereComponent false))
      (bind _output_get_2 (Variables|Default|SetRightHandAttackSphere _returnvalue_2))
      (Transformation|AttachComponentToComponent _output_get_2 (Variables|Character|GetMesh) "RightHandSocket" "SnapToTarget" "SnapToTarget" "KeepRelative" true))))

(fn SetDead
  (params (Normal :type Vector) (Speed :type Float%20%28single-precision%29))
  (bind _returnvalue (Game|GetGameMode))
  (bind _returnvalue_2 (Game|GetGameMode))
  (Variables|Default|SetisAttacking false)
  (Variables|Default|SetIsDead? true)
  (Class|PhysicalAnimationComponent|SetStrengthMultiplyer (Variables|Default|GetPhysicalAnimation) 0.0)
  (Physics|SetSimulatePhysics (Variables|Character|GetMesh) true)
  (Collision|SetCollisionEnabled (Variables|Collision|GetCapsuleComponent) "NoCollision")
  (Collision|SetCollisionEnabled (Variables|Default|GetRightHandAttackSphere) "NoCollision")
  (Class|Pawn|DetachfromControllerPendingDestroy)
  (bind _asfps_waves_game_mode (Utilities|Casting|CastToFPS_WavesGameMode _returnvalue)
    (:then
      (Variables|/Game/Blueprints/FPS_WavesGameMode.FPS_WavesGameMode_C|SetPlayerScore _asfps_waves_game_mode (+ (Variables|/Game/Blueprints/FPS_WavesGameMode.FPS_WavesGameMode_C|GetPlayerScore _asfps_waves_game_mode) (Variables|Default|GetScore))))
    (:CastFailed
      (bind _asfpsc___waves_game_mode (Utilities|Casting|CastToFPSC++_WavesGameMode _returnvalue))
      (Variables|/Game/Blueprints/FPSC++_WavesGameMode.FPSC++_WavesGameMode_C|SetPlayerScore _asfpsc___waves_game_mode (+ (Variables|/Game/Blueprints/FPSC++_WavesGameMode.FPSC++_WavesGameMode_C|GetPlayerScore _asfpsc___waves_game_mode) (Variables|Default|GetScore)))))
  (bind _asfps_waves_game_mode_2 (Utilities|Casting|CastToFPS_WavesGameMode _returnvalue_2)
    (:then
      (Default|CheckIsAllDead _asfps_waves_game_mode_2))
    (:CastFailed
      (bind _asfpsc___waves_game_mode_2 (Utilities|Casting|CastToFPSC++_WavesGameMode _returnvalue_2))
      (Default|CheckIsAllDead _asfpsc___waves_game_mode_2)))
  (Actor|SetLifeSpan 1e+01)
  (Default|AddXP (Actor|GetComponentbyClass (Game|GetPlayerCharacter 0) "/Game/Blueprints/StatSystem/BP_BaseStatComponent.BP_BaseStatComponent_C") (Variables|Default|GetAddingXP)))