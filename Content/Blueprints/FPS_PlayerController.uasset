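; First-person shooter player controller that turns input into movement, look, jump and weapon fire for FPS_PlayerCharacter.
; InitWaveMode caches the controlled pawn as that character, switches to game-only input with a hidden cursor, and adds the UI_WaveModPlayer widget to the viewport.
; Movement and jump act on the cached character, look axes feed controller pitch and yaw, and Fire pulls or releases the trigger on the character's TommyRef.
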(event Custom|InitWaveMode
  (bind _returnvalue (Pawn|GetControlledPawn))
  (bind (_asfps_player_character _bsuccess) (Utilities|Casting|CastToFPS_PlayerCharacter _returnvalue))
  (if _bsuccess
    (Variables|Default|SetPlayerCharacter _asfps_player_character)
    (Input|SetInputModeGameOnly self)
    (Variables|Default|SetbShowMouseCursor false)
    (bind _returnvalue_2 (UserInterface|CreateWidget "/Game/UI/UI_WaveModPlayer.UI_WaveModPlayer_C" self))
    (bind _output_get (Variables|Default|SetWaveUI _returnvalue_2))
    (UserInterface|Viewport|AddtoViewport _output_get 0)))

(event Input|ActionEvents|InputActionJump
  (params (Key :type Key%20Structure))
  (:Pressed
    (Character|Jump (Variables|Default|GetPlayerCharacter))))

(event Input|ActionEvents|InputActionFire
  (params (Key :type Key%20Structure))
  (bind _playercharacter (Variables|Default|GetPlayerCharacter))
  (bind _tommyref (Variables|/Game/Blueprints/FPS_PlayerCharacter.FPS_PlayerCharacter_C|GetTommyRef _playercharacter))
  (:Pressed
    (Default|PullTrigger _tommyref))
  (:Released
    (Default|ReleaseTrigger _tommyref)))

(event Input|AxisEvents|InputAxisMoveUp
  (params (AxisValue :type Float%20%28single-precision%29))
  (Pawn|Input|AddMovementInput (Variables|Default|GetPlayerCharacter) (Transformation|GetActorForwardVector (Variables|Default|GetPlayerCharacter)) AxisValue false))

(event Input|AxisEvents|InputAxisMoveRight
  (params (AxisValue :type Float%20%28single-precision%29))
  (Pawn|Input|AddMovementInput (Variables|Default|GetPlayerCharacter) (Transformation|GetActorRightVector (Variables|Default|GetPlayerCharacter)) AxisValue false))

(event Input|AxisEvents|InputAxisLookUp
  (params (AxisValue :type Float%20%28single-precision%29))
  (Class|PlayerController|AddPitchInput AxisValue))

(event Input|AxisEvents|InputAxisLookRight
  (params (AxisValue :type Float%20%28single-precision%29))
  (Class|PlayerController|AddYawInput AxisValue))

(fn ConstructionScript)