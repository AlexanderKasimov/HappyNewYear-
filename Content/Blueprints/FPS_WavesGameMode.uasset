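; Game mode for a wave-based FPS that spawns growing waves of enemies through the level's WaveSpawner actors.
; A one-second countdown timer raises the enemy count and wave number, then gives each spawner a quarter of the total, implicitly assuming four spawners.
; CheckIsAllDead recounts living enemies and restarts the countdown at zero, while another timer trims old blood decals.
; PlayerDead is empty, and the death-screen logic is unconnected.
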(event Custom|WaveCountDown
  (bind _output_get (Variables|Default|SetCountDownTime (- (Variables|Default|GetCountDownTime) 1.0)))
  (if (<= _output_get 0.0)
    (Variables|Default|SetStartWaveEnemyCount (+ (Variables|Default|GetStartWaveEnemyCount) (Variables|Default|GetWaveIncrementValue)))
    (Math|Integer|IncrementInt (Variables|Default|GetCurWave)
      (:%20%20
        (Variables|Default|SetAliveEnemyCount (Variables|Default|GetStartWaveEnemyCount))
        (CallFunction|SpawnWave)
        (if (Utilities|Time|IsValidTimerHandle (stale EventBeginPlay _returnvalue))
          (Utilities|Time|ClearandInvalidateTimerbyHandle (stale EventBeginPlay _returnvalue))
          (Variables|Default|SetCountDownTime (Variables|Default|GetMaxCountDownTime))
          (else
            (Utilities|Time|ClearandInvalidateTimerbyHandle (stale Custom|CheckIsAllDead _returnvalue))
            (Variables|Default|SetCountDownTime (Variables|Default|GetMaxCountDownTime))))))))

(event Custom|ClearDecals
  (bind _blooddecalarray (Variables|Default|GetBloodDecalArray))
  (bind _output (Utilities|Array|Get(acopy) _blooddecalarray))
  (if (>= (Utilities|Array|Length (Variables|Default|GetBloodDecalArray)) 200)
    (for _index (range 1 3)
      (Components|DestroyComponent _output)
      (Utilities|Array|RemoveItem (Variables|Default|GetBloodDecalArray) _output))))

(event Custom|CheckIsAllDead
  (Variables|Default|SetAliveEnemyIterator 0)
  (bind _outactors (Actor|GetAllActorsOfClass "/Game/Blueprints/EnemyCharacter.EnemyCharacter_C"))
  (for _array_element _outactors
    (if (not (Variables|/Game/Blueprints/EnemyCharacter.EnemyCharacter_C|GetIsDead? _array_element))
      (Math|Integer|IncrementInt (Variables|Default|GetAliveEnemyIterator))))
  (bind _output_get (Variables|Default|SetAliveEnemyCount (Variables|Default|GetAliveEnemyIterator)))
  (if (not (> _output_get 0))
    (bind _returnvalue (Utilities|Time|SetTimerbyEvent (delegate Custom|WaveCountDown) 1.0 true))))

(event Custom|PlayerDead)

(event Custom|SpawnWave
  (for _array_element (Variables|Default|GetWaveSpawnersArray)
    (Default|SpawnWave _array_element (/ (Variables|Default|GetStartWaveEnemyCount) 4))))

(event EventBeginPlay
  (bind _asfps_player_controller (Utilities|Casting|CastToFPS_PlayerController (Game|GetPlayerController 0)))
  (bind _output_get (Variables|Default|SetPlayerController _asfps_player_controller))
  (Default|InitWaveMode _output_get)
  (bind _outactors (Actor|GetAllActorsOfClass "/Game/Blueprints/WaveSpawner.WaveSpawner_C"))
  (for _array_element _outactors
    (bind _aswave_spawner (Utilities|Casting|CastToWaveSpawner _array_element))
    (Utilities|Array|Add (Variables|Default|GetWaveSpawnersArray) _aswave_spawner))
  (bind _returnvalue (Utilities|Time|SetTimerbyEvent (delegate Custom|WaveCountDown) 1.0 true))
  (Utilities|Time|SetTimerbyEvent (delegate Custom|ClearDecals) 2.0 true))

(fn ConstructionScript)