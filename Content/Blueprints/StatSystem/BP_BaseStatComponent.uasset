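; Base actor component for character stats: health, fatigue, XP and leveling, and movement speed.
; On BeginPlay it derives max HP from Endurance, fills HP and fatigue, loads the XP requirement from a level DataTable and adds a Speed-based bonus to the owner's walk speed.
; AddXP loops through level-ups, granting skill points and refreshing the requirement from the table, while ProcessDamage subtracts from current HP without clamping.
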(event EventBeginPlay
  (CallFunction|CalculateHP)
  (CallFunction|InitFatigue)
  (CallFunction|InitXP)
  (CallFunction|CalculateMovementSpeed))

(event EventTick
  (params (DeltaSeconds :type Float%20%28single-precision%29)))

(fn InitHealth
  (Variables|Default|SetCurHP (Variables|Default|GetMaxHP)))

(fn ProcessDamage
  (params (Damage :type Float%20%28single-precision%29))
  (Variables|Default|SetCurHP (- (Variables|Default|GetCurHP) Damage)))

(fn AddXP
  (params (AddedXP :type Float%20%28single-precision%29))
  (LocalVariables|SetLocalAddedXP AddedXP)
  (Variables|Default|SetCurXP (+ (Variables|Default|GetCurXP) (LocalVariables|GetLocalAddedXP)))
  (while (>= (Variables|Default|GetCurXP) (Variables|Default|GetReqXP))
    (Variables|Default|SetCurXP (- (Variables|Default|GetCurXP) (Variables|Default|GetReqXP)))
    (Math|Integer|IncrementInt (Variables|Default|GetLVL)
      (:%20%20
        (Math|Integer|IncrementInt (Variables|Default|GetSkillPoints)
          (:%20%20
            (bind _returnvalue (Utilities|GetDataTableRow "/Game/Blueprints/StatSystem/LVL_List_DT.LVL_List_DT" (Utilities|String|StringToName (Utilities|String|ToString(Integer) (- (Variables|Default|GetLVL) 1))))
              (:then
                (Variables|Default|SetReqXP (Utilities|Struct|BreakLVL_List_Struct _returnvalue))))))))))

(fn InitXP
  (bind _returnvalue (Utilities|GetDataTableRow "/Game/Blueprints/StatSystem/LVL_List_DT.LVL_List_DT" (Utilities|String|StringToName (Utilities|String|ToString(Integer) (- (Variables|Default|GetLVL) 1))))
    (:then
      (Variables|Default|SetReqXP (Utilities|Struct|BreakLVL_List_Struct _returnvalue)))))

(fn InitFatigue
  (Variables|Default|SetCurFatigue (Variables|Default|GetMaxFatigue)))

(fn CalculateMovementSpeed
  (bind _returnvalue (Components|GetOwner))
  (bind _returnvalue_2 (Actor|GetComponentbyClass _returnvalue "/Script/Engine.CharacterMovementComponent"))
  (Utilities|IsValid _returnvalue_2
    (:Is%20Valid
      (bind _output_get (LocalVariables|SetMovementComponent _returnvalue_2))
      (Variables|/Script/Engine.CharacterMovementComponent|SetMaxWalkSpeed _output_get (+ (Math|Float|MapRangeClamped (Variables|Default|GetSpeed) 0.0 1e+02 0.0 4e+02) (Variables|/Script/Engine.CharacterMovementComponent|GetMaxWalkSpeed _output_get))))))

(fn CalculateHP
  (Variables|Default|SetMaxHP (* (Variables|Default|GetEndurance) 2.0))
  (CallFunction|InitHealth))