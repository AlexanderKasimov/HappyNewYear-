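; Tommy gun bullet actor that deals damage and plays an impact sound when its mesh overlaps another actor.
; For IDamagable actors, a short PhysicsBody line trace through the bullet recovers a hit result, which it sends with damage and speed to the traced actor.
; A successful trace plays a flesh sound and destroys the bullet, while a miss leaves it alive.
; Other actors trigger a dirt sound and destroy it.
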(event OnComponentBeginOverlap(BulletMesh)
  (params (OverlappedComponent :type Primitive%20Component%20Object%20Reference) (OtherActor :type Actor%20Object%20Reference) (OtherComp :type Primitive%20Component%20Object%20Reference) (OtherBodyIndex :type Integer) (bFromSweep :type Boolean) (SweepResult :type Hit%20Result%20Structure%20%28by%20ref%29))
  (bind _returnvalue (Transformation|GetActorRotation))
  (bind _bulletmesh (Variables|Default|GetBulletMesh))
  (bind _returnvalue_2 (Transformation|GetWorldLocation _bulletmesh))
  (bind _returnvalue_3 (Math|Vector|GetForwardVector _returnvalue))
  (Development|PrintString (Utilities|GetDisplayName OtherActor))
  (if (Utilities|DoesObjectImplementInterface OtherActor "/Game/Blueprints/iDamagable.iDamagable_C")
    (bind (_outhit _returnvalue_4) (Collision|LineTraceForObjects (+ _returnvalue_2 (* _returnvalue_3 -1e+02)) (+ _returnvalue_2 (* _returnvalue_3 1e+02)) (Utilities|Array|MakeArray "ObjectTypeQuery4") true 0 "None"))
    (if _returnvalue_4
      (Class|IDamagable|RecieveDamage(Message) (.HitActor (Collision|BreakHitResult _outhit)) _outhit (Variables|Default|GetDamage) (Math|Vector|VectorLength (Transformation|GetVelocity)))
      (Audio|PlaySoundatLocation "/Game/Sound/InGameSound/bullet_flesh_mega_Cue.bullet_flesh_mega_Cue" (.Location (Collision|BreakHitResult _outhit)))
      (Actor|DestroyActor))
    (else
      (Audio|PlaySoundatLocation "/Game/Sound/InGameSound/Impact_Dirt_20_Cue.Impact_Dirt_20_Cue" (Transformation|GetActorLocation))
      (Actor|DestroyActor))))

(event EventBeginPlay
  (|CallParentFunction) ; This node is disabled and will not be called.\nDrag off pins to build functionality.
)

(event Collision|EventActorBeginOverlap
  (params (OtherActor :type Actor%20Object%20Reference))
  (|CallParentFunction OtherActor) ; This node is disabled and will not be called.\nDrag off pins to build functionality.
)

(event EventTick
  (params (DeltaSeconds :type Float%20%28single-precision%29))
  (|CallParentFunction DeltaSeconds) ; This node is disabled and will not be called.\nDrag off pins to build functionality.
)

(fn ConstructionScript
  (|CallParentFunction))