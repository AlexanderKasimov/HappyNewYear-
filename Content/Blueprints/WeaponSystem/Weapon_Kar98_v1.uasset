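; Kar98 weapon Blueprint that fires one shot per trigger pull, rate-limited by a timer that resets a DoOnce.
; Fire line-traces from the muzzle toward the player camera's aim point, with debug drawing, prints and placeholder-like Thompson sounds.
; Hits on IDamagable actors receive fixed damage after a distance-based delay that simulates bullet travel, using a hardcoded speed.
; Firing on an empty magazine starts a timed reload.
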(event Custom|AllowFire
  (Utilities|FlowControl|DoOnce false) ; enters at Reset
)

(event Custom|CustomEvent_0)

(event EventPullTrigger
  (Utilities|FlowControl|DoOnce false
    (:Completed
      (CallFunction|Fire)
      (bind _returnvalue (Utilities|Time|SetTimerbyEvent (delegate Custom|AllowFire) (/ 6e+01 (Variables|Default|GetFireRate))))
      (Variables|Default|SetFireTimer _returnvalue))))

(event EventReleaseTrigger)

(event EventFire
  (bind _returnvalue (Game|GetPlayerController 0))
  (bind _range (Variables|Default|GetRange))
  (bind _bulletspawn (Variables|Components|GetBulletSpawn))
  (bind _returnvalue_2 (Transformation|GetWorldLocation _bulletspawn))
  (bind (_outlocation _outrotation) (Actor|GetActorEyesViewPoint _returnvalue))
  (bind _returnvalue_3 (Math|Rotator|GetRotationXVector _outrotation))
  (bind _returnvalue_4 (* _returnvalue_3 _range))
  (bind _returnvalue_5 (+ _outlocation _returnvalue_4))
  (if (> (Variables|Default|GetCurAmmoInMagazine) 0)
    (Development|PrintString (Utilities|String|ToString(Vector) _returnvalue_5))
    (bind (_outhit _returnvalue_6) (Collision|LineTraceByChannel _returnvalue_2 _returnvalue_5 "TraceTypeQuery1" true 0 "ForDuration"))
    (Math|Integer|DecrementInt (Variables|Default|GetCurAmmoInMagazine)
      (:%20%20
        (Audio|PlaySoundatLocation "/Game/Sound/InGameSound/thompson_01_Cue.thompson_01_Cue" (.Location (Math|Transform|BreakTransform (Transformation|GetWorldTransform _bulletspawn))))
        (if _returnvalue_6
          (if (Utilities|DoesObjectImplementInterface (.HitActor (Collision|BreakHitResult _outhit)) "/Game/Blueprints/iDamagable.iDamagable_C")
            (Development|PrintString (Utilities|String|ToString(Float) (Math|Vector|VectorLength (- (.Location (Collision|BreakHitResult _outhit)) _returnvalue_2))))
            (Utilities|FlowControl|Delay (/ (Math|Vector|VectorLength (- (.Location (Collision|BreakHitResult _outhit)) _returnvalue_2)) (* 2.8e+02 1e+02)))
            (Class|IDamagable|RecieveDamage(Message) (.HitActor (Collision|BreakHitResult _outhit)) _outhit 5e+01 (Variables|Default|GetBulletSpeed))))))
    (else
      (Utilities|FlowControl|DoOnce false
        (:Completed
          (Utilities|Time|SetTimerbyEvent (delegate EventReload) (Variables|Default|GetReloadTime))
          (Audio|PlaySoundatLocation "/Game/Sound/InGameSound/thompson_reload_Cue.thompson_reload_Cue" (Transformation|GetWorldLocation (Variables|Default|GetDefaultSceneRoot))))))))

(event EventReload
  (Variables|Default|SetCurAmmoInMagazine (Variables|Default|GetMagazineSize))
  (Utilities|FlowControl|DoOnce false) ; enters at Reset
)

(event EventBeginPlay
  (Variables|Default|SetCurAmmoInMagazine (Variables|Default|GetMagazineSize)))

(fn ConstructionScript
  (|CallParentFunction))