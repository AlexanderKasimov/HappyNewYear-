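; Tommy gun weapon Blueprint that fires automatically on a looping fire-rate timer while the trigger is held.
; Each shot line-traces forward from BulletSpawn with debug drawing, spends ammo and plays a sound.
; Hits on IDamagable actors send damage after a distance-based delay that mimics bullet travel time.
; Firing on an empty clip starts a timed reload with sound; an AmmoType spawn node is left unconnected.
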(event EventPullTrigger
  (Utilities|FlowControl|DoOnce false
    (:Completed
      (CallFunction|Fire)
      (bind _returnvalue (Utilities|Time|SetTimerbyEvent (delegate EventFire) (/ 6e+01 (Variables|Default|GetFireRate)) true))
      (Variables|Default|SetFireTimer _returnvalue))))

(event EventReleaseTrigger
  (Utilities|Time|ClearandInvalidateTimerbyHandle (Variables|Default|GetFireTimer))
  (Utilities|FlowControl|DoOnce false) ; enters at Reset
)

(event EventFire
  (bind _bulletspawn (Variables|Components|GetBulletSpawn))
  (bind _returnvalue (Transformation|GetWorldLocation _bulletspawn))
  (if (> (Variables|Default|GetCurAmmo) 0)
    (bind (_outhit _returnvalue_2) (Collision|LineTraceByChannel _returnvalue (+ _returnvalue (* (Math|Vector|GetForwardVector _bulletspawn) (Variables|Default|GetRange))) "TraceTypeQuery1" true 0 "ForDuration"))
    (Math|Integer|DecrementInt (Variables|Default|GetCurAmmo)
      (:%20%20
        (Audio|PlaySoundatLocation "/Game/Sound/InGameSound/thompson_01_Cue.thompson_01_Cue" (.Location (Math|Transform|BreakTransform (Transformation|GetWorldTransform _bulletspawn))))
        (if _returnvalue_2
          (if (Utilities|DoesObjectImplementInterface (.HitActor (Collision|BreakHitResult _outhit)) "/Game/Blueprints/iDamagable.iDamagable_C")
            (Development|PrintString (Utilities|String|ToString(Float) (Math|Vector|VectorLength (- (.Location (Collision|BreakHitResult _outhit)) _returnvalue))))
            (Utilities|FlowControl|Delay (/ (Math|Vector|VectorLength (- (.Location (Collision|BreakHitResult _outhit)) _returnvalue)) (* 2.8e+02 1e+02)))
            (Class|IDamagable|RecieveDamage(Message) (.HitActor (Collision|BreakHitResult _outhit)) _outhit 3e+01 (Variables|Default|GetBulletSpeed))))))
    (else
      (Utilities|FlowControl|DoOnce false
        (:Completed
          (Utilities|Time|SetTimerbyEvent (delegate EventReload) (Variables|Default|GetReloadTime))
          (Audio|PlaySoundatLocation "/Game/Sound/InGameSound/thompson_reload_Cue.thompson_reload_Cue" (Transformation|GetWorldLocation (Variables|Default|GetDefaultSceneRoot))))))))

(event EventReload
  (Variables|Default|SetCurAmmo (Variables|Default|GetClipSize))
  (Utilities|FlowControl|DoOnce false) ; enters at Reset
)

(event EventBeginPlay
  (Variables|Default|SetCurAmmo (Variables|Default|GetClipSize)))

(fn ConstructionScript
  (|CallParentFunction))